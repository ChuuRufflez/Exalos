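; Base item actor that the player can interact with, with a helper for adding it to the inventory.
; BeginPlay caches the MainPlayerController and disables input, which is then enabled only while a MainPlayerCharacter overlaps the actor.
; Pressing Interact calls the Interacted event, left empty here.
; AddToPlayerInventory passes the item name and a given amount to the MainPlayerController's AddToInventory.
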(event `self.ReceiveBeginPlay`
  (bind _asmain_player_controller (cast `/Game/Blueprints/Character/MainPlayerController` (`GameplayStatics.GetPlayerController` 0)))
  (set `self.Player` _asmain_player_controller)
  (`self.DisableInput` (`GameplayStatics.GetPlayerController` 0)))

(event `self.ReceiveActorBeginOverlap`
  (params (OtherActor :type "Actor Object Reference"))
  (cast `/Game/Blueprints/Character/MainPlayerCharacter` OtherActor)
  (`self.EnableInput` (`GameplayStatics.GetPlayerController` 0)))

(event `InputAction|Interact`
  (params (Key :type "Key Structure"))
  (:`Pressed`
    (`self.Interacted`)))

(event `self.ReceiveActorEndOverlap`
  (params (OtherActor :type "Actor Object Reference"))
  (cast `/Game/Blueprints/Character/MainPlayerCharacter` OtherActor)
  (`self.DisableInput` (`GameplayStatics.GetPlayerController` 0)))

(event `Interacted`)

(fn `addToPlayerInventory`
  (params (amountToAdd :type Integer))
  (bind _asmain_player_controller (cast `/Game/Blueprints/Character/MainPlayerController` (`GameplayStatics.GetPlayerController` 0)))
  (`/Game/Blueprints/Character/MainPlayerController.addToInventory` _asmain_player_controller (`self.itemName`) amountToAdd))

(fn `UserConstructionScript`)