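; MainPlayerController is the player controller that handles character input, the toolbar HUD and the player's inventory.
; Axis inputs move and rotate MainPlayerCharacter, while holding right mouse yaws its spring arm from mouse X on Tick.
; BeginPlay creates the toolbar, shows the cursor and caches widget references, with an input action toggling the inventory.
; AddToInventory stacks matching item names, uses a gate to append new ones, and refreshes the inventory list.
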(event `RefreshInventory`
  (bind _widget_inventory (`self.Widget_Inventory`))
  (`PanelWidget.ClearChildren` (`/Game/Blueprints/UI/Widget_Inventory.ScrollBox_InventoryList` _widget_inventory))
  (`/Game/Blueprints/UI/Widget_Inventory.List Items` _widget_inventory))

(event `InputAxis|Vertical Input`
  (params (AxisValue :type "Float (single-precision)"))
  ;[1 1 1] Player movement
  (bind _asmain_player_character (cast `/Game/Blueprints/Character/MainPlayerCharacter` (`GameplayStatics.GetPlayerCharacter` 0)))
  (`/Game/Blueprints/Character/MainPlayerCharacter.MoveForward` _asmain_player_character AxisValue))

(event `self.ReceiveBeginPlay`
  ;[1 1 1] Adding HUDWidget to viewport
  (bind _returnvalue (`|CreateWidget` "/Game/Blueprints/UI/Widget_ToolBar.Widget_ToolBar_C" self))
  (`UserWidget.AddToViewport` _returnvalue 0)
  (set `self.bShowMouseCursor` true)
  (bind _foundwidgets (`WidgetBlueprintLibrary.GetAllWidgetsOfClass` "/Game/Blueprints/UI/Widget_Inventory.Widget_Inventory_C" false))
  (set `self.Widget_Inventory` (`|GetArrayItem` _foundwidgets))
  (bind _foundwidgets_2 (`WidgetBlueprintLibrary.GetAllWidgetsOfClass` "/Game/Blueprints/UI/Widget_ToolBar.Widget_ToolBar_C" false))
  (set `self.Widget_ToolBar` (`|GetArrayItem` _foundwidgets_2))
  (bind _asmain_player_character (cast `/Game/Blueprints/Character/MainPlayerCharacter` (`GameplayStatics.GetPlayerCharacter` 0)))
  (set `self.MainPlayerCharacter` _asmain_player_character))

(event `InputAxis|Horizontal Input`
  (params (AxisValue :type "Float (single-precision)"))
  ;[1 1 1] Player movement
  (bind _asmain_player_character (cast `/Game/Blueprints/Character/MainPlayerCharacter` (`GameplayStatics.GetPlayerCharacter` 0)))
  (`/Game/Blueprints/Character/MainPlayerCharacter.RotatePlayer` _asmain_player_character AxisValue))

(event `self.ReceiveTick`
  (params (DeltaSeconds :type "Float (single-precision)"))
  (if (`self.rightMousePressed`)
    (`SceneComponent.K2_AddWorldRotation` (`/Game/Blueprints/Character/MainPlayerCharacter.SpringArm` (`self.MainPlayerCharacter`)) (`KismetMathLibrary.MakeRotator` 0.0 0.0 (* (`self.GetInputAxisValue`) 2.0)) false false)))

(event `InputAction|Show Inventory`
  (params (Key :type "Key Structure"))
  (:`Pressed`
    (`/Game/Blueprints/UI/Widget_ToolBar.Show/Hide Inventory` (`self.Widget_ToolBar`))))

(event `Key|RightMouseButton`
  (params (Key :type "Key Structure"))
  (:`Pressed`
    (set `self.rightMousePressed` true))
  (:`Released`
    (set `self.rightMousePressed` false)))

(fn `addToInventory`
  (params (itemName :type Name) (amountToAdd :type Integer))
  (bind _inventorystruct (`self.InventoryStruct`))
  (for (_array_element _array_index) _inventorystruct
    (bind (_itemname _itemamount) (break `/Game/Blueprints/Character/Inventory` _array_element))
    (if (== itemName _itemname)
      (`|ExecutionSequence`
        (:`then_0`
          (`KismetArrayLibrary.Array_Set` _inventorystruct _array_index (make `/Game/Blueprints/Character/Inventory` itemName (+ _itemamount amountToAdd)))
          (`|ExecutionSequence`
            (:`then_0`
              (goto _label :!via `Close`))
            (:`then_1`
              (`self.RefreshInventory`))))
        (:`then_1`
          (break)))))
  (`/Engine/EditorBlueprintResources/StandardMacros.Gate` false :!label _label
    (:`Exit`
      (`KismetArrayLibrary.Array_Add` _inventorystruct (make `/Game/Blueprints/Character/Inventory` itemName amountToAdd))
      (`self.RefreshInventory`))))

(fn `UserConstructionScript`)